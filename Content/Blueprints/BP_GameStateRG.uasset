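; BP_GameStateRG is a game state Blueprint that tracks contestants, finished players and dead players, and shows the pre-game and game-over screens.
; BeginPlay binds an event to OnGameStateUpdated, and the CreateWidget event adds either the pre-game or game-over widget to the viewport based on GameStart.
; RepNotify functions fire dispatchers: contestant changes call OnUpdatePlayerCount, while finished and dead name changes both call OnUpdateFinishedPlayers.
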(event `self.ReceiveBeginPlay`
  (add `self.OnGameStateUpdated` (`|CreateDelegate` :!event `CreateWidget`)))

(event `CreateWidget` :!signature `self.OnGameStateUpdated`
  (params (bGameStart :type Boolean))
  (if bGameStart
    (bind _returnvalue (`|CreateWidget` "/Game/Blueprints/Widgets/Widget_PreGame.Widget_PreGame_C"))
    (`UserWidget.AddToViewport` _returnvalue 0)
    (else
      (bind _returnvalue_2 (`|CreateWidget` "/Game/Blueprints/Widgets/Widget_GameOver.Widget_GameOver_C"))
      (`UserWidget.AddToViewport` _returnvalue_2 0))))

(fn `OnRep_Contestants`
  (`self.OnUpdatePlayerCount`))

(fn `OnRep_DeadPlayerNames`
  (`self.OnUpdateFinishedPlayers`))

(fn `OnRep_FinishedPlayerNames`
  (`self.OnUpdateFinishedPlayers`))

(fn `UserConstructionScript`)