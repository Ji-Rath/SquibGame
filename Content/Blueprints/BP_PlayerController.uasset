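; Player controller that toggles a pause menu widget on the Pause input action.
; If the stored widget is on screen, it removes it, re-enables look input and sets cursor visibility from the look-ignore state.
; Otherwise it creates a new Widget_Pause, adds it to the viewport and stores the reference.
; Opening the menu changes neither game pause, input nor cursor state here.
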(event `InputAction|Pause`
  (params (Key :type "Key Structure"))
  (:`Pressed`
    (`/Engine/EditorBlueprintResources/StandardMacros.IsValid` (`self.PauseWidget`)
      (:`Is Valid`
        (if (`Widget.IsInViewport` (`self.PauseWidget`))
          (`Widget.RemoveFromParent` (`self.PauseWidget`))
          (`self.SetIgnoreLookInput` false)
          (set `self.bShowMouseCursor` (`self.IsLookInputIgnored`))
          (else
            (bind _returnvalue (`|CreateWidget` "/Game/Blueprints/Widgets/Widget_Pause.Widget_Pause_C" self :!label _label))
            (`UserWidget.AddToViewport` _returnvalue 0)
            (set `self.PauseWidget` _returnvalue))))
      (:`Is Not Valid`
        (goto _label)))))

(fn `UserConstructionScript`)