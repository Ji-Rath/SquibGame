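; BP_SpectateCamera is a spectator camera that follows active players, with Turn and LookUp input rotating the view.
; On BeginPlay and each player-count update from BP_GameStateRG, it rebuilds its contestant list from BP_Player actors that can move, then switches target.
; Pressing Roll also advances through the list with wraparound, attaching the camera by snapping location and keeping relative rotation.
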(event `InputAxis|LookUp`
  (params (AxisValue :type "Float (single-precision)"))
  (`self.AddControllerPitchInput` AxisValue))

(event `InputAxis|Turn`
  (params (AxisValue :type "Float (single-precision)"))
  (`self.AddControllerYawInput` AxisValue))

(event `self.ReceiveBeginPlay`
  (bind _asbp_game_state_rg (cast `/Game/Blueprints/BP_GameStateRG` (`GameplayStatics.GetGameState`)))
  (add `/Game/Blueprints/BP_GameStateRG.OnUpdatePlayerCount` _asbp_game_state_rg (delegate `UpdateContestants`))
  (`self.UpdateContestants`))

(event `UpdateContestants`
  (`KismetArrayLibrary.Array_Clear` (`self.Contestants`))
  (bind _outactors (`GameplayStatics.GetAllActorsOfClass` "/Game/Blueprints/BP_Player.BP_Player_C"))
  (for _array_element _outactors
    (bind _returnvalue (`HumanCharacter.CanMove` _array_element))
    (if _returnvalue
      (`KismetArrayLibrary.Array_Add` (`self.Contestants`) _array_element)))
  (`self.SpectatePlayer`))

(event `InputAction|Roll`
  (params (Key :type "Key Structure"))
  (:`Pressed`
    (`self.SpectatePlayer`)))

(fn `CheckSpectator`
  (if (>= (`self.CurrentSpectator`) (`KismetArrayLibrary.Array_Length` (`self.Contestants`)))
    (set `self.CurrentSpectator` 0)))

(fn `SpectatePlayer`
  (bind _output (`|GetArrayItem` (`self.Contestants`) (`self.CurrentSpectator`)))
  (`self.CheckSpectator`)
  (`/Engine/EditorBlueprintResources/StandardMacros.IsValid` _output
    (:`Is Valid`
      (`self.K2_AttachToActor` _output "None" "SnapToTarget" "KeepRelative" "KeepRelative")
      (`/Engine/EditorBlueprintResources/StandardMacros.IncrementInt` (`self.CurrentSpectator`)))
    (:`Is Not Valid`
      (`/Engine/EditorBlueprintResources/StandardMacros.IncrementInt` (`self.CurrentSpectator`)))))

(fn `UserConstructionScript`)