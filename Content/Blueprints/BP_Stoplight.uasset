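; BP_Stoplight is a stoplight actor that shows whether the game is in a green-light or red-light state through its point light.
; On BeginPlay it binds an event to OnGameStart on BP_GamemodeRG, though the bound handler's logic is not shown.
; Every Tick it sets the light to green or red from IsGreenLight, which nothing in these graphs changes.
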(event `self.ReceiveBeginPlay`
  (bind _asbp_gamemode_rg (cast `/Game/Blueprints/BP_GamemodeRG` (`GameplayStatics.GetGameMode`)))
  (add `/Game/Blueprints/BP_GamemodeRG.OnGameStart` _asbp_gamemode_rg (`|CreateDelegate` :!event `BeginLightTimer`)))

(event `self.ReceiveTick`
  (params (DeltaSeconds :type "Float (single-precision)"))
  (bind _pointlight (`self.PointLight`))
  (if (`self.bIsGreenLight`)
    (`LightComponent.SetLightColor` _pointlight (`KismetMathLibrary.LinearColor_Green`) true)
    (else
      (`LightComponent.SetLightColor` _pointlight (`KismetMathLibrary.LinearColor_Red`) true))))

(fn `UserConstructionScript`)