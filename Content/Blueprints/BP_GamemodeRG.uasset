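; BP_GamemodeRG is a game mode that runs a timed match in which characters play until each has finished.
; StartGame flags the game state as started, starts a looping one-second countdown, fires OnGameStart and registers every Character as a contestant.
; Each countdown tick copies the reduced time limit to BP_GameStateRG.
; PlayerFinish records successful finishers, removes the contestant and shows the Game Over widget once none remain.
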(fn `Player Finish`
  (params (Finisher :type "Actor Object Reference") (bSuccess :type Boolean))
  (bind _contestants (`self.Contestants`))
  (if bSuccess
    (`KismetArrayLibrary.Array_Add` (`self.FinishedPlayers`) Finisher))
  (`KismetArrayLibrary.Array_RemoveItem` _contestants Finisher)
  (if (<= (`KismetArrayLibrary.Array_Length` _contestants) 0)
    (bind _returnvalue (`|CreateWidget` "/Game/Blueprints/Widgets/Widget_GameOver.Widget_GameOver_C"))
    (`UserWidget.AddToViewport` _returnvalue 0)))

(fn `StartGame`
  (bind _asbp_game_state_rg (cast `/Game/Blueprints/BP_GameStateRG` (`GameplayStatics.GetGameState`)))
  (set `/Game/Blueprints/BP_GameStateRG.bGameStarted` true _asbp_game_state_rg)
  (`KismetSystemLibrary.K2_SetTimer` null "SubtractTime" 1.0 true)
  (`self.OnGameStart`)
  (bind _outactors (`GameplayStatics.GetAllActorsOfClass` "/Script/Engine.Character"))
  (set `self.Contestants` _outactors))

(fn `SubtractTime`
  (bind _output_get (set `self.TimeLimit` (- (`self.TimeLimit`) (`KismetMathLibrary.MakeTimespan` 0 0 0 1))))
  (bind _asbp_game_state_rg (cast `/Game/Blueprints/BP_GameStateRG` (`GameplayStatics.GetGameState`)))
  (set `/Game/Blueprints/BP_GameStateRG.TimeLimit` _output_get _asbp_game_state_rg))

(fn `UserConstructionScript`)